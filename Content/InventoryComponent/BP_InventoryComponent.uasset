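; BP_InventoryComponent is an inventory component that stores picked-up items by class and shows them in a widget.
; Show and hide functions create or remove the four-column widget for the local player, switching input mode and cursor unless Controller is set.
; Adding an item plays a pickup sound, either in 2D or replicated at the item's location through server and multicast events.
; The server and client item-spawn functions are empty stubs.
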(event `Server_PlaySound`
  (params (Sound :type "SoundBase Object Reference") (Location :type "Vector Structure"))
  (`self.MC_PlaySound` Sound Location))

(event `MC_PlaySound`
  (params (Sound :type "SoundBase Object Reference") (Location :type "Vector Structure"))
  (`GameplayStatics.PlaySoundAtLocation` Sound Location (struct) 1.0 1.0 0.0 null null null null))

(fn `Client_SpawnItem`
  (params (Class1 :type "Actor Object Reference") (SpawnTransform1 :type "Transform Structure")))

(fn `F_AddItemToInventory`
  (params (NewItem :type "/Game/InventoryComponent/BP_MasterItem Object Reference (by ref)"))
  (bind _returnvalue (`SceneComponent.K2_GetComponentLocation` (`/Game/InventoryComponent/BP_MasterItem.StaticMesh` NewItem)))
  (`KismetArrayLibrary.Array_Add` (`self.Inventory`) (`GameplayStatics.GetObjectClass` NewItem))
  (if (`self.ReplicatePickupSound?`)
    (`/Engine/EditorBlueprintResources/ActorComponentMacros.Switch Has Authority`
      (:`Authority`
        (`self.MC_PlaySound` "/Game/StarterContent/Audio/Explosion01.Explosion01" _returnvalue))
      (:`Remote`
        (`self.Server_PlaySound` "/Game/StarterContent/Audio/Explosion01.Explosion01" _returnvalue)))
    (else
      (`GameplayStatics.PlaySound2D` "/Game/StarterContent/Audio/Explosion01.Explosion01" 1.0 1.0 0.0 null null))))

(fn `F_HideInventory`
  (`/Engine/EditorBlueprintResources/StandardMacros.IsValid` (`self.BP_Inventory`)
    (:`Is Valid`
      (`Widget.RemoveFromParent` (`self.BP_Inventory`))
      (if (not (`self.Controller?`))
        (`WidgetBlueprintLibrary.SetInputMode_GameOnly` (`GameplayStatics.GetPlayerController` 0))
        (set `PlayerController.bShowMouseCursor` false (`GameplayStatics.GetPlayerController` 0))))))

(fn `F_ShowInventory`
  (bind _returnvalue (`GameplayStatics.GetPlayerController` 0))
  (if (`Controller.IsLocalPlayerController` _returnvalue)
    (bind _returnvalue_2 (`|CreateWidget` "/Game/InventoryComponent/WB_Inventorywidget.WB_Inventorywidget_C" _returnvalue))
    (bind _output_get (set `self.BP_Inventory` _returnvalue_2))
    (`UserWidget.AddToViewport` _output_get 0)
    (`/Game/InventoryComponent/WB_Inventorywidget.F_Update` _returnvalue_2 (`self.Inventory`) "NewEnumerator0" null null null)
    (if (not (`self.Controller?`))
      (`WidgetBlueprintLibrary.SetInputMode_GameAndUIEx` (`GameplayStatics.GetPlayerController` 0) (`self.BP_Inventory`) "LockInFullscreen")
      (set `PlayerController.bShowMouseCursor` true (`GameplayStatics.GetPlayerController` 0)))))

(fn `Server_SpawnItem`
  (params (Class1 :type "Actor Class Reference") (SpawnTransform1 :type "Transform Structure")))